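; Mover component that shifts and rotates its owning actor between its starting pose and an offset pose.
; BeginPlay derives both targets and constant speeds from the offsets and MoveTime, and ActivateMover enables Tick to interpolate toward them.
; On arrival each channel snaps and swaps start and target, reversing the next movement.
; A gate opened by location arrival and entered by rotation arrival disables ticking.
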(event `self.ReceiveBeginPlay`
  (bind _returnvalue (`self.GetOwner`))
  (bind _returnvalue_2 (`Actor.K2_GetActorLocation` _returnvalue))
  (bind _returnvalue_3 (`Actor.K2_GetActorRotation` _returnvalue))
  (`|ExecutionSequence`
    (:`then_0`
      ;[0.9823 0.5776 0.01681] Location
      (bind _output_get (set `self.Local Starting Location` _returnvalue_2))
      (bind _output_get_2 (set `self.Local Target Location` (+ (`self.Move Offset`) _returnvalue_2)))
      (set `self.Local Move Speed` (/ (`KismetMathLibrary.Vector_Distance` _output_get_2 _output_get) (`self.Move Time`))))
    (:`then_1`
      ;[0.3419 0.4452 0.9734] Rotation
      (bind _output_get_3 (set `self.Local Starting Rotation` _returnvalue_3))
      (bind _output_get_4 (set `self.Local Target Rotation` (`KismetMathLibrary.ComposeRotators` (`self.Rotate Offset`) _returnvalue_3)))
      (bind (_returnvalue_roll _returnvalue_pitch _returnvalue_yaw) (`KismetMathLibrary.BreakRotator` (`KismetMathLibrary.NormalizedDeltaRotator` _output_get_4 _output_get_3)))
      (set `self.Rotate Speed` (/ (`KismetMathLibrary.VSize` (`KismetMathLibrary.MakeVector` _returnvalue_roll _returnvalue_pitch _returnvalue_yaw)) (`self.Move Time`))))))

(event `self.ReceiveTick`
  (params (DeltaSeconds :type "Float (single-precision)"))
  (bind _returnvalue (`self.GetOwner`))
  (bind _local_target_location (`self.Local Target Location`))
  (bind _local_target_rotation (`self.Local Target Rotation`))
  (bind _returnvalue_2 (`Actor.K2_GetActorRotation` _returnvalue))
  (bind _returnvalue_3 (`Actor.K2_GetActorLocation` _returnvalue))
  (`|ExecutionSequence`
    (:`then_0`
      ;[0.9823 0.5776 0.01681] Location
      (`Actor.K2_SetActorLocation` _returnvalue (`KismetMathLibrary.VInterpTo_Constant` _returnvalue_3 (`self.Local Target Location`) DeltaSeconds (`self.Local Move Speed`)) false false)
      (if (== _returnvalue_3 _local_target_location :`ErrorTolerance` 1e-05)
        (`Actor.K2_SetActorLocation` _returnvalue _local_target_location false true) ; Force Target Location
        (`self.Swap Move Direction`)
        (goto _label :!via `Open`)))
    (:`then_1`
      ;[0.3419 0.4452 0.9734] Rotation
      (`Actor.K2_SetActorRotation` _returnvalue (`KismetMathLibrary.RInterpTo_Constant` _returnvalue_2 (`self.Local Target Rotation`) DeltaSeconds (`self.Rotate Speed`)) false)
      (if (== _returnvalue_2 _local_target_rotation :`ErrorTolerance` 1e-05)
        (`Actor.K2_SetActorRotation` _returnvalue _local_target_rotation false)
        (`self.Swap Rotate Direction`)
        ;[1 1 1] Esegue solo se entrambe le execution line sono partite.
        (`/Engine/EditorBlueprintResources/StandardMacros.Gate` true :!label _label
          (:`Exit`
            (`self.SetComponentTickEnabled` false)
            (goto _label :!via `Close`)))))))

(event `Activate Mover`
  (`self.SetComponentTickEnabled` true))

(fn `Swap Move Direction`
  (locals (`Local Temp` :type "Vector Structure"))
  (set `local.Local Temp` (`self.Local Target Location`))
  (set `self.Local Target Location` (`self.Local Starting Location`))
  (set `self.Local Starting Location` (`local.Local Temp`)))

(fn `Swap Rotate Direction`
  (locals (`Local Temp` :type "Rotator Structure"))
  (set `local.Local Temp` (`self.Local Target Rotation`))
  (set `self.Local Target Rotation` (`self.Local Starting Rotation`))
  (set `self.Local Starting Rotation` (`local.Local Temp`)))