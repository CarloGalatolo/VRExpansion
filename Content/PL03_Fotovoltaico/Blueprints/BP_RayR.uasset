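; BP_RayR is a VR hand laser pointer for interacting with 3D buttons, which destroys itself outside the safe-space maps.
; Each Tick it line-traces to its HitPoint, sizing the Niagara beam and placing a sphere at any hit.
; It tracks the hit actor to send hover on and off through BP_InteractionComponent.
; TryInteraction, called by VRCharacter, forwards presses with the owning hand to that component.
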(event `self.ReceiveBeginPlay`
  ;[1 1 1] Shoud be visible only in starting map
  (if (not (or (`/Game/PL03_Fotovoltaico/Blueprints/Libraries/BPFL_Game.Is Current Level` "L_SafeSpace") (`/Game/PL03_Fotovoltaico/Blueprints/Libraries/BPFL_Game.Is Current Level` "L_MYSafeSpace")))
    (`self.K2_DestroyActor`) ; Avoids calling Tick uselessly.
  ))

(event `self.ReceiveTick`
  (params (DeltaSeconds :type "Float (single-precision)"))
  (bind _owning_hand (`self.Owning Hand`))
  (bind _returnvalue (`self.GetComponentByClass` (`self.Actual Hit Actor`) "/Game/PL03_Fotovoltaico/Blueprints/Components/BP_InteractionComponent.BP_InteractionComponent_C"))
  ;[1 1 1] Check if hitting a 3D Button
  (bind _outhit (`KismetSystemLibrary.LineTraceSingle` (`self.K2_GetActorLocation`) (`SceneComponent.K2_GetComponentLocation` (`self.Hit Point`)) "TraceTypeQuery3" false (`|MakeArray` (`GameplayStatics.GetPlayerPawn` 0) :!type "Actor Object Reference")))
  (`self.On Actor Hit` (`.Distance` (`GameplayStatics.BreakHitResult` _outhit)) (`.Location` (`GameplayStatics.BreakHitResult` _outhit)) (`GameplayStatics.BreakHitResult` _outhit))
  (if (`GameplayStatics.BreakHitResult` _outhit)
    (bind _actual_hit_actor (`self.Actual Hit Actor`)
      (:`then`
        (if (== _actual_hit_actor (`.HitActor` (`GameplayStatics.BreakHitResult` _outhit)))
          (`/Game/PL03_Fotovoltaico/Blueprints/Components/BP_InteractionComponent.On Hover` _returnvalue true _owning_hand :!label _label)
          (else
            (`|ExecutionSequence`
              (:`then_0`
                (`/Game/PL03_Fotovoltaico/Blueprints/Components/BP_InteractionComponent.On Hover` _returnvalue false _owning_hand :!label _label_2)
                (set `self.Actual Hit Actor` null) ; Clear
              )
              (:`then_1`
                (set `self.Actual Hit Actor` (`.HitActor` (`GameplayStatics.BreakHitResult` _outhit)) :!label _label_3)
                (goto _label))))))
      (:`else`
        (goto _label_3)))
    (else
      (`self.Actual Hit Actor`
        (:`then`
          (goto _label_2))
        (:`else`)))))

(event `Try Interaction`
  (params (Pressed :type Boolean))
  ;[1 1 1] Interact with buttons
  (bind _actual_hit_actor (`self.Actual Hit Actor`)
    (:`then`
      (`/Game/PL03_Fotovoltaico/Blueprints/Components/BP_InteractionComponent.On Press` (`self.GetComponentByClass` _actual_hit_actor "/Game/PL03_Fotovoltaico/Blueprints/Components/BP_InteractionComponent.BP_InteractionComponent_C") Pressed (`self.Owning Hand`)))
    (:`else`)))

(fn `On Actor Hit`
  (params (`Hit Distance` :type "Float (double-precision)") (NewLocation :type "Vector Structure") (`Actor Hit` :type Boolean))
  (bind _sphere (`self.Sphere`))
  (`NiagaraComponent.SetVariableVec3` (`self.NS_Ray`) "Beam End" (`KismetMathLibrary.MakeVector` (`KismetMathLibrary.SelectFloat` `Hit Distance` 100.0 `Actor Hit`)))
  (`SceneComponent.SetHiddenInGame` _sphere (not `Actor Hit`) false)
  (`SceneComponent.K2_SetWorldLocation` _sphere NewLocation false false))

(fn `UserConstructionScript`)