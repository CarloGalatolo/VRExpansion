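; Blueprint function library with shared helpers for a guided VR tour.
; It checks the current level name and reads the guide flag from BP_MYGameInstance.
; On authority, GuideAdvanceTour resets the player 0 VR character's interaction Do Once, increments the tour phase in BP_GameInstance and copies it to BP_GameState.
; The guide check and phase advance cast to differently named game instance classes.
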(fn `Guide Advance Tour`
  (bind ___worldcontext (`local.__WorldContext`))
  (bind _returnvalue (`GameplayStatics.GetPlayerCharacter` ___worldcontext))
  (if (`Actor.HasAuthority` _returnvalue)
    (bind _asbp_vrcharacter (cast `/Game/PL03_Fotovoltaico/Blueprints/Game/BP_VRCharacter` _returnvalue))
    (`/Game/PL03_Fotovoltaico/Blueprints/Game/BP_VRCharacter.Tour Interaction Reset` _asbp_vrcharacter) ; Resets Do Once on BP_VRCharacter
    ;[0.0137 0.7605 0.4233] Next Tour Phase
    (bind _result (`/Engine/EditorBlueprintResources/StandardMacros.IncrementInt` (`/Game/PL03_Fotovoltaico/Blueprints/Game/BP_GameInstance.Instance Tour Phase` (cast `/Game/PL03_Fotovoltaico/Blueprints/Game/BP_GameInstance` (`GameplayStatics.GetGameInstance` ___worldcontext) :!pure true)))
      (:`  `
        (set `/Game/PL03_Fotovoltaico/Blueprints/Game/BP_GameState.Tour Phase` _result (cast `/Game/PL03_Fotovoltaico/Blueprints/Game/BP_GameState` (`GameplayStatics.GetGameState` ___worldcontext) :!pure true))))))

(fn `Is Current Level`
  (params (`Level Name` :type String))
  (returns (`Is Current Level` :type Boolean))
  (bind _returnvalue (`GameplayStatics.GetCurrentLevelName` (`local.__WorldContext`)))
  (return (== _returnvalue `Level Name`)))

(fn `Is Guide`
  (returns (`Instance Is Guide` :type Boolean))
  (return (`/Game/Developers/Carlo/BP_MYGameInstance.Instance Is Guide` (cast `/Game/Developers/Carlo/BP_MYGameInstance` (`GameplayStatics.GetGameInstance` (`local.__WorldContext`)) :!pure true))))