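; Abstract VRE grippable base for long objects that can be gripped anywhere along their length in VR.
; It overrides ClosestGripSlotInRange to snap the grip to the closest point on the GripLine spline.
; The slot is always reported as in range, using the spline component's world rotation, unit scale and its object name as slot name.
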(fn `ClosestGripSlotInRange`
  (params (WorldLocation :type "Vector Structure") (bSecondarySlot :type Boolean) (CallingController :type "GripMotionControllerComponent Object Reference") (OverridePrefix :type Name))
  (returns (bHadSlotInRange :type Boolean) (SlotWorldTransform :type "Transform Structure") (SlotName :type Name))
  (locals (`Local ClosestSplinePoint` :type "Vector Structure"))
  (bind _gripline (`self.GripLine`))
  ;[0.9647 0.5711 0.01681] Finds nearest point in the Grip Spline
  (set `local.Local ClosestSplinePoint` (`SplineComponent.FindLocationClosestToWorldLocation` (`self.GripLine`) WorldLocation "World"))
  ;[0.2623 0.02956 0.3712] Returns the transform to be set when gripping.
  (return true (`KismetMathLibrary.MakeTransform` (`local.Local ClosestSplinePoint`) (`SceneComponent.K2_GetComponentRotation` _gripline)) (`KismetStringLibrary.Conv_StringToName` (`KismetSystemLibrary.GetObjectName` _gripline))) ; Grip is slotted.
)

(fn `UserConstructionScript`
  (`parent.UserConstructionScript`))