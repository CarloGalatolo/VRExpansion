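; A grippable VR lever component that rotates about its roll axis to follow the gripping motion controller.
; Each grip tick converts the controller into the lever's initial frame on its attach parent and applies the atan2 angle change since grab.
; The grip authority drops it beyond the break distance.
; On release it can tick back at constant speed to its start or target roll, and GetAngle reports the current angle.
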(event `self.ReceiveBeginPlay`
  (bind _relativerotation_roll (`KismetMathLibrary.BreakRotator` (`self.RelativeRotation`)))
  (set `self.InitialRot` _relativerotation_roll)
  (set `self.InitialTransform` (`self.GetRelativeTransform`)))

(event `self.OnGrip`
  (params (GrippingController :type "GripMotionControllerComponent Object Reference") (GripInformation :type "BPActorGripInformation Structure (by ref)"))
  (bind _relativerotation_roll (`KismetMathLibrary.BreakRotator` (`self.RelativeRotation`)))
  (set `self.bIsLerping` false)
  (bind _output_get (set `self.InteractingController` GrippingController))
  (set `self.RotAtGrab` _relativerotation_roll)
  (bind _returnvalue (`KismetMathLibrary.InverseTransformLocation` (`self.GetCurTransform`) (`self.K2_GetComponentLocation` _output_get)))
  (set `self.InitialInteractorLocation` _returnvalue)
  (bind (_returnvalue_x _returnvalue_y) (`KismetMathLibrary.BreakVector` (`KismetMathLibrary.LessLess_VectorRotator` _returnvalue (struct :`Pitch` 90.0))))
  (set `self.InitialGripRot` (`KismetMathLibrary.DegAtan2` _returnvalue_y _returnvalue_x)))

(event `self.OnGripRelease`
  (params (ReleasingController :type "GripMotionControllerComponent Object Reference") (GripInformation :type "BPActorGripInformation Structure (by ref)") (bWasSocketed :type Boolean))
  (if (`self.ReturnAfterRelease`)
    (set `self.bIsLerping` true)
    (`self.SetComponentTickEnabled` true)
    (else
      (`self.SetComponentTickEnabled` false))))

(event `self.ReceiveTick`
  (params (DeltaSeconds :type "Float (single-precision)"))
  (bind (_relativerotation_roll _relativerotation_pitch _relativerotation_yaw) (`KismetMathLibrary.BreakRotator` (`self.RelativeRotation`)))
  (bind _returnvalue (`KismetMathLibrary.SelectFloat` (`self.InitialRot`) (`self.TargetRot`) (`self.Lerp To Start`)))
  (bind _returnvalue_2 (`KismetMathLibrary.FInterpTo_Constant` _relativerotation_roll _returnvalue DeltaSeconds (`self.ReturnSpeed`)))
  ;[0.03955 0.6514 0] Interp back to position
  (if (`self.bIsLerping`)
    (`self.K2_SetRelativeRotation` (`KismetMathLibrary.MakeRotator` _returnvalue_2 _relativerotation_pitch _relativerotation_yaw))
    (if (`KismetMathLibrary.NearlyEqual_FloatFloat` _returnvalue_2 _returnvalue)
      (set `self.bIsLerping` false)
      (`self.SetComponentTickEnabled` false))))

(event `VRGripInterface.TickGrip`
  (params (GrippingController :type "GripMotionControllerComponent Object Reference") (GripInformation :type "BPActorGripInformation Structure (by ref)") (DeltaTime :type "Float (single-precision)"))
  (bind (_relativerotation_roll _relativerotation_pitch _relativerotation_yaw) (`KismetMathLibrary.BreakRotator` (`self.RelativeRotation`)))
  (bind (_vrgripinterfacesettings_bdenygripping _vrgripinterfacesettings_ballowmultiplegrips _vrgripinterfacesettings_onteleportbehavior _vrgripinterfacesettings_bsimulateondrop _vrgripinterfacesettings_slotdefaultgriptype _vrgripinterfacesettings_freedefaultgriptype _vrgripinterfacesettings_secondarygriptype _vrgripinterfacesettings_movementreplicationtype _vrgripinterfacesettings_lateupdatesetting _vrgripinterfacesettings_constraintstiffness _vrgripinterfacesettings_constraintdamping _vrgripinterfacesettings_constraintbreakdistance) (break `BPInterfaceProperties` (`self.VRGripInterfaceSettings`)))
  (bind _returnvalue (`KismetMathLibrary.InverseTransformLocation` (`self.GetCurTransform`) (`self.K2_GetComponentLocation` GrippingController)))
  (bind (_returnvalue_x _returnvalue_y) (`KismetMathLibrary.BreakVector` (`KismetMathLibrary.LessLess_VectorRotator` _returnvalue (struct :`Pitch` 90.0))))
  (if (and (>= (`KismetMathLibrary.VSize` (- _returnvalue (`self.InitialInteractorLocation`))) _vrgripinterfacesettings_constraintbreakdistance) (`GripMotionControllerComponent.BP_HasGripAuthority` GrippingController GripInformation))
    (`GripMotionControllerComponent.DropObjectByInterface` GrippingController self 0 (0.0 0.0 0.0) (0.0 0.0 0.0)) ; Drop it, we are out of range
    (else
      (`self.K2_SetRelativeRotation` (`KismetMathLibrary.MakeRotator` (+ (`self.RotAtGrab`) (- (`KismetMathLibrary.DegAtan2` _returnvalue_y _returnvalue_x) (`self.InitialGripRot`))) _relativerotation_pitch _relativerotation_yaw)))))

(fn `GetAngle`
  (returns (`Current Angle From Start` :type "Float (double-precision)") (`Actual Angle` :type "Float (double-precision)"))
  (bind _relativerotation_roll (`KismetMathLibrary.BreakRotator` (`self.RelativeRotation`)))
  (return (- _relativerotation_roll (`self.InitialRot`)) _relativerotation_roll))

(fn `GetCurTransform`
  (returns (Transform :type "Transform Structure"))
  (return (`KismetMathLibrary.ComposeTransforms` (`self.InitialTransform`) (`self.K2_GetComponentToWorld` (`self.GetAttachParent`)))))